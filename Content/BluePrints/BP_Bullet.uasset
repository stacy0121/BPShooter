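; BP_Bullet is a projectile actor that flies straight along world up and destroys itself after a short lifespan.
; BeginPlay sets Direction to the positive Z axis and starts the lifespan timer.
; Tick moves the actor by normalized Direction times Speed and delta time, using a swept SetActorLocation so blocking geometry stops the movement.
; The file contains no hit or damage logic, as the overlap event is disabled.
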(event `self.ReceiveBeginPlay`
  ;[1 1 1] 전역 변수로
  (set `self.Direction` (`KismetMathLibrary.MakeVector` 0.0 0.0 1.0))
  (`self.SetLifeSpan` 2.0))

(event `self.ReceiveTick`
  (params (DeltaSeconds :type "Float (single-precision)"))
  ;[1 1 1] vt
  (`self.K2_SetActorLocation` (+ (* (* (`KismetMathLibrary.Normal` (`self.Direction`)) (`self.Speed`)) DeltaSeconds) (`self.K2_GetActorLocation`)) true))

(fn `UserConstructionScript`)