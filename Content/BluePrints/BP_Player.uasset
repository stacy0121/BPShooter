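; BP_Player is the player actor, which moves in the Y-Z plane and shoots bullets.
; Horizontal and Vertical axis inputs share one Direction setter, and Tick normalizes that vector, scales it by Speed and delta time, then moves the actor with sweep.
; BeginPlay enables input from player controller 0.
; Pressing Fire calls ShootBullet, which spawns BP_Bullet at the actor's transform and plays a 2D sound.
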(event `self.ReceiveBeginPlay`
  ;[1 1 1] 시작해서 입력 가능케
  (`self.EnableInput` (`GameplayStatics.GetPlayerController` 0)))

(event `InputAxis|Horizontal`
  (params (AxisValue :type "Float (single-precision)"))
  (set `self.Direction` (`KismetMathLibrary.MakeVector` 0.0 AxisValue (stale `InputAxis|Vertical` AxisValue)) :!label _label))

(event `InputAxis|Vertical`
  (params (AxisValue :type "Float (single-precision)"))
  (goto _label))

(event `self.ReceiveTick`
  (params (DeltaSeconds :type "Float (single-precision)"))
  ;[1 1 1] P0 + vt
  ;[1 1 1] P
  (`self.K2_SetActorLocation` (+ (* (* (`KismetMathLibrary.Normal` (`self.Direction`)) (`self.Speed`)) DeltaSeconds) (`self.K2_GetActorLocation`)) true))

(event `InputAction|Fire`
  (params (Key :type "Key Structure"))
  (:`Pressed`
    ;[1 1 1] 총알을 만들고 싶다.
    (`self.ShootBullet`)))

(fn `ShootBullet`
  (`|SpawnActorFromClass` "/Game/BluePrints/BP_Bullet.BP_Bullet_C" (`self.GetTransform`) "AlwaysSpawn" "OverrideRootScale" null null)
  ;[1 1 1] audio component와 같다
  (`GameplayStatics.PlaySound2D` "/Game/Sounds/Audio_Bullet.Audio_Bullet" 1.0 1.0 0.0 null null))

(fn `UserConstructionScript`)