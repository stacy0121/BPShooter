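; BP_Enemy is an enemy actor that flies in a straight line and destroys itself along with whatever it hits.
; On BeginPlay it finds BP_Player, and FindDirection randomly picks either the direction toward the player or straight down, the fallback without a valid target.
; Tick moves it along that fixed direction with a swept location update.
; Box overlap plays explosion sound and particles, then destroys both actors without a type check.
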(event `self.ReceiveBeginPlay`
  ;[1 1 1] BP_Player 설계도로 만들어진 액터를 찾아서 Target 변수에 넣음(동적)
  (bind _returnvalue (`GameplayStatics.GetActorOfClass` "/Game/BluePrints/BP_Player.BP_Player_C"))
  (set `self.Target` _returnvalue)
  (`self.FindDirection`))

(event `self.ReceiveTick`
  (params (DeltaSeconds :type "Float (single-precision)"))
  ;[1 1 1] 원하는 방향으로 이동
  ;;[1 1 1] P
  (`self.K2_SetActorLocation` (+ (* (* (`self.Direction`) (`self.Speed`)) DeltaSeconds) (`self.K2_GetActorLocation`)) true))

(event `self.StaticMesh.OnComponentBeginOverlap`
  (params (OverlappedComponent :type "PrimitiveComponent Object Reference") (OtherActor :type "Actor Object Reference") (OtherComp :type "PrimitiveComponent Object Reference") (OtherBodyIndex :type Integer) (bFromSweep :type Boolean) (SweepResult :type "HitResult Structure (by ref)")))

(event `self.Box.OnComponentBeginOverlap`
  (params (OverlappedComponent :type "PrimitiveComponent Object Reference") (OtherActor :type "Actor Object Reference") (OtherComp :type "PrimitiveComponent Object Reference") (OtherBodyIndex :type Integer) (bFromSweep :type Boolean) (SweepResult :type "HitResult Structure (by ref)"))
  ;[1 1 1] 부딪혔을 때 너죽고 나죽자(other actor : 부딪힌 대상) - 단, 적이 아니라면(명시적 형변환 type casting)
  (`GameplayStatics.PlaySound2D` "/Game/Sounds/Audio_Explosion.Audio_Explosion" 1.0 1.0 0.0 null null)
  (`GameplayStatics.SpawnEmitterAtLocation` "/Game/StarterContent/Particles/P_Explosion.P_Explosion" (`self.K2_GetActorLocation`))
  (`self.K2_DestroyActor` OtherActor)
  (`self.K2_DestroyActor`))

(event `self.ReceiveActorBeginOverlap`
  (params (OtherActor :type "Actor Object Reference"))
  ;[1 1 1] 부딪혔을 때(너죽고 나죽자)
)

(fn `FindDirection`
  (bind _target (`self.Target`))
  ;[1 1 1] 유효하면
  (if (`KismetSystemLibrary.IsValid` _target)
    ;[1 1 1] 50보다 작으면 내 쪽으로
    (if (< (`KismetMathLibrary.RandomIntegerInRange` 1 100) 50)
      (set `self.Direction` (`KismetMathLibrary.Normal` (- (`self.K2_GetActorLocation` _target) (`self.K2_GetActorLocation`))))
      (else
        (set `self.Direction` (0.0 0.0 -1.0) :!label _label)))
    (else
      (goto _label))))

(fn `UserConstructionScript`)